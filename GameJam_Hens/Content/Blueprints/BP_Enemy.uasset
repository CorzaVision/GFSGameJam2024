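; BP_Enemy is an enemy creature that the player can kill or capture with projectiles, depending on the player's active mode.
; Damage mode subtracts projectile damage from Health, destroying the enemy at zero.
; Capture mode destroys it immediately, adds a soul to the weapon component, and has a delayed re-show of the player's Sphere queued after destruction.
; Touching the player only prints a damage message, throttled by a two-second cooldown.
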(event Collision|EventHit
  (params (MyComp :type Primitive%20Component%20Object%20Reference) (Other :type Actor%20Object%20Reference) (OtherComp :type Primitive%20Component%20Object%20Reference) (bSelfMoved :type Boolean) (HitLocation :type Vector :default "0, 0, 0") (HitNormal :type Vector :default "0, 0, 0") (NormalImpulse :type Vector :default "0, 0, 0") (Hit :type Hit%20Result%20Structure%20%28by%20ref%29))
  (bind _fp (Variables|Default|GetFP))
  (bind _fp_2 (Variables|Default|GetFP))
  (Utilities|FlowControl|Sequence
    (:then_0
      ;[1 1 1] Destroy Once Projectile Hits
      (bind _asbp_first_person_projectile (Utilities|Casting|CastToBP_FirstPersonProjectile Other))
      (Variables|Default|SetProjectile _asbp_first_person_projectile)
      (Development|PrintString "Actor has been Hit")
      (Utilities|FlowControl|Sequence
        (:then_0
          (if (Variables|/Game/FirstPerson/Blueprints/BP_FirstPersonCharacter.BP_FirstPersonCharacter_C|GetDamage%20Mode _fp_2)
            (CallFunction|Damage)
            (if (<= (Variables|Default|GetHealth) 0)
              (Actor|DestroyActor)
              (Variables|Default|SetHit%20Actor false)
              (Development|PrintString "Creature has Been Killed"))))
        (:then_1
          (if (Variables|/Game/FirstPerson/Blueprints/BP_FirstPersonCharacter.BP_FirstPersonCharacter_C|GetCapture%20Mode _fp_2)
            (Actor|DestroyActor)
            (Variables|Default|SetHit%20Actor false)
            (Development|PrintString "Creature has Been Captured")
            (Default|AddASoul (Variables|/Game/FirstPerson/Blueprints/BP_FirstPersonCharacter.BP_FirstPersonCharacter_C|GetBP_Weapon_Component _fp))
            (Utilities|FlowControl|Delay 3.0)
            (Rendering|SetVisibility (Variables|/Game/FirstPerson/Blueprints/BP_FirstPersonCharacter.BP_FirstPersonCharacter_C|GetSphere _fp) true false)))))
    (:then_1
      ;[1 1 1] Hit Player
      (Utilities|Casting|CastToBP_FirstPersonCharacter Other)
      (if (not (Variables|Default|GetHit%20Player))
        (Development|PrintString "DAMAGE ACTOR !!!" true true "(R=1.000000,G=0.008781,B=0.000000,A=1.000000)")
        (Variables|Default|SetHit%20Player true)
        (Utilities|FlowControl|Delay 2.0)
        (Variables|Default|SetHit%20Player false)))))

(event EventBeginPlay
  (bind _asbp_first_person_character (Utilities|Casting|CastToBP_FirstPersonCharacter (Game|GetPlayerCharacter 0)))
  (Variables|Default|SetFP _asbp_first_person_character))

(fn ConstructionScript)

(fn Damage
  (bind _output_get (Variables|Default|SetHealth (- (Variables|Default|GetHealth) (Variables|/Game/FirstPerson/Blueprints/BP_FirstPersonProjectile.BP_FirstPersonProjectile_C|GetProjectile%20Damage (Variables|Default|GetProjectile)))))
  (Development|PrintString (Utilities|String|ToString(Integer) _output_get) true true "(R=0.253266,G=1.000000,B=0.215784,A=1.000000)"))