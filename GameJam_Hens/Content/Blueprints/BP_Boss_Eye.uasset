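; Boss eye enemy that shoots at the player and can be killed or captured with the first-person projectile.
; Projectile hits either subtract Health or roll a weighted capture chance awarding a soul, depending on the player's damage or capture mode.
; Attack waits, spawns a boss projectile aimed at the player's mesh from an arrow offset, then signals attack end.
; Player contact only prints a damage message, throttled by a flag and delay.
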(event Collision|EventHit
  (params (MyComp :type Primitive%20Component%20Object%20Reference) (Other :type Actor%20Object%20Reference) (OtherComp :type Primitive%20Component%20Object%20Reference) (bSelfMoved :type Boolean) (HitLocation :type Vector :default "0, 0, 0") (HitNormal :type Vector :default "0, 0, 0") (NormalImpulse :type Vector :default "0, 0, 0") (Hit :type Hit%20Result%20Structure%20%28by%20ref%29))
  (bind _fp (Variables|Default|GetFP))
  (bind _fp_2 (Variables|Default|GetFP))
  (Utilities|FlowControl|Sequence
    (:then_0
      ;[1 1 1] Destroy Once Projectile Hits
      (bind _asbp_first_person_projectile (Utilities|Casting|CastToBP_FirstPersonProjectile Other))
      (Variables|Default|SetProjectile _asbp_first_person_projectile)
      (Development|PrintString "Actor has been Hit")
      (Utilities|FlowControl|Sequence
        (:then_0
          (if (Variables|/Game/FirstPerson/Blueprints/BP_FirstPersonCharacter.BP_FirstPersonCharacter_C|GetDamage%20Mode _fp_2)
            (Utilities|FlowControl|DoOnce false :!label _label
              (:Completed
                (CallFunction|Damage)
                (if (<= (Variables|Default|GetHealth) 0)
                  (Actor|DestroyActor)
                  (Variables|Default|SetHit%20Actor false)
                  (Development|PrintString "Creature has Been Killed")
                  (goto _label Reset)
                  (else
                    (goto _label Reset)))))))
        (:then_1
          (if (Variables|/Game/FirstPerson/Blueprints/BP_FirstPersonCharacter.BP_FirstPersonCharacter_C|GetCapture%20Mode _fp_2)
            (if (Variables|Default|GetCanBeCaptured)
              (Utilities|FlowControl|DoOnce false :!label _label_2
                (:Completed
                  (if (Math|Random|RandomBoolwithWeight (Variables|Default|GetCaptureRate))
                    (Actor|DestroyActor)
                    (Variables|Default|SetHit%20Actor false)
                    (Development|PrintString "Creature has Been Captured")
                    (Default|AddASoul (Variables|/Game/FirstPerson/Blueprints/BP_FirstPersonCharacter.BP_FirstPersonCharacter_C|GetBP_Weapon_Component _fp))
                    (Utilities|FlowControl|Delay 3.0)
                    (Rendering|SetVisibility (Variables|/Game/FirstPerson/Blueprints/BP_FirstPersonCharacter.BP_FirstPersonCharacter_C|GetSphere _fp) true false)
                    (goto _label_2 Reset)
                    (else
                      (Development|PrintString "FAILED TO CAPTURE" true true "(R=0.609699,G=0.000000,B=1.000000,A=1.000000)")
                      (goto _label_2 Reset)))))
              (else
                (Development|PrintString "Creature Cannot Be Captured" true true "(R=1.000000,G=0.042624,B=0.000000,A=1.000000)")))))))
    (:then_1
      ;[1 1 1] Hit Player
      (Utilities|Casting|CastToBP_FirstPersonCharacter Other)
      (if (not (Variables|Default|GetHit%20Player))
        (Development|PrintString "DAMAGE ACTOR !!!" true true "(R=1.000000,G=0.008781,B=0.000000,A=1.000000)")
        (Variables|Default|SetHit%20Player true)
        (Utilities|FlowControl|Delay 2.0)
        (Variables|Default|SetHit%20Player false)))))

(event EventBeginPlay
  (bind _asbp_first_person_character (Utilities|Casting|CastToBP_FirstPersonCharacter (Game|GetPlayerCharacter 0)))
  (Variables|Default|SetFP _asbp_first_person_character))

(event Custom|Attack
  (Utilities|FlowControl|Delay 1.0)
  (CallFunction|SpawnProjectile)
  (Development|PrintString "BOSS PROJECTILE SPAWNED" true true "(R=0.442472,G=0.000000,B=1.000000,A=1.000000)")
  (Default|CallOnAttackEnd))

(event Custom|Spawn%20Projectile
  (bind _projectilearrow (Variables|Default|GetProjectileArrow))
  (bind _returnvalue (Transformation|GetWorldLocation _projectilearrow))
  (Game|SpawnActorfromClass "/Game/Blueprints/BP_Boss_Projectile.BP_Boss_Projectile_C" (Math|Transform|MakeTransform (+ _returnvalue (Math|Vector|RotateVector (Variables|Default|GetProjectileOffset) (Transformation|GetWorldRotation _projectilearrow))) (Math|Rotator|FindLookatRotation _returnvalue (Transformation|GetWorldLocation (Variables|/Script/Engine.Character|GetMesh (Game|GetPlayerCharacter 0))))) "Undefined" "MultiplyWithRoot" 0 0))

(fn ConstructionScript)

(fn Damage
  (bind _output_get (Variables|Default|SetHealth (- (Variables|Default|GetHealth) (Variables|/Game/FirstPerson/Blueprints/BP_FirstPersonProjectile.BP_FirstPersonProjectile_C|GetProjectile%20Damage (Variables|Default|GetProjectile)))))
  (Development|PrintString (Utilities|String|ToString(Integer) _output_get) true true "(R=0.253266,G=1.000000,B=0.215784,A=1.000000)"))